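; Locked double-door prop that the player opens with the Mahjong1 inventory item (the Dragon piece).
; Entering the key-check collision shows the locked text; finding the piece also enables input, shows the HUD door text and opens a Gate.
; Pressing E through that Gate removes the piece and destroys the collision and both door meshes rather than animating them.
; Leaving the collision disables input, hides both texts and closes the Gate.
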(event `Key|E`
  (params (Key :type "Key Structure"))
  ;[1 1 1] Locked Door
  (:`Pressed`
    (`/Engine/EditorBlueprintResources/StandardMacros.Gate` true :!label _label
      (:`Exit`
        (bind _asthird_person_character (cast `/Game/OAH/OAH_Blueprint/Player/ThirdPersonCharacter` (`GameplayStatics.GetPlayerCharacter` 0)))
        (bind _inventoryarray (`/Game/OAH/OAH_Blueprint/Player/ThirdPersonCharacter.InventoryArray` _asthird_person_character))
        (for _array_element _inventoryarray :!label _label_2
          (if (`KismetTextLibrary.EqualEqual_TextText` (`.ItemName_9_D15C36564F6449EF98FB6CB521D23004` (break `/Game/OAH/OAH_Blueprint/Player/InventorySystem/ItemStructure/Struct_ItemStruct` _array_element)) (`self.Mahjong_1`))
            (`self.KeyRemoved`)
            (bind _returnvalue (`KismetArrayLibrary.Array_RemoveItem` _inventoryarray _array_element))
            (if _returnvalue
              (bind _asthird_person_character_2 (cast `/Game/OAH/OAH_Blueprint/Player/ThirdPersonCharacter` (`GameplayStatics.GetPlayerCharacter` 0)))
              (`/Game/OAH/OAH_Widget/HUDWidget.Show Door Text` (`/Game/OAH/OAH_Blueprint/Player/ThirdPersonCharacter.HUD` _asthird_person_character_2) false)
              (`ActorComponent.K2_DestroyComponent` (`self.collision_KeyCheck`))
              (`SceneComponent.K2_SetRelativeRotation` (`self.mesh_DoorRight`) (`KismetMathLibrary.MakeRotator` 0.0) false false)
              (`ActorComponent.K2_DestroyComponent` (`self.mesh_DoorLeft`))
              (`ActorComponent.K2_DestroyComponent` (`self.mesh_DoorRight`)))))))))

(event `KeyRemoved`
  ;[1 1 1] Locked Door
  (goto _label_2 :!via `Break`))

(event `self.collision_KeyCheck.OnComponentBeginOverlap`
  (params (OverlappedComponent :type "PrimitiveComponent Object Reference") (OtherActor :type "Actor Object Reference") (OtherComp :type "PrimitiveComponent Object Reference") (OtherBodyIndex :type Integer) (bFromSweep :type Boolean) (SweepResult :type "HitResult Structure (by ref)"))
  ;[1 1 1] Locked Door
  (`SceneComponent.SetVisibility` (`self.text_Locked`) true false)
  (bind _asthird_person_character (cast `/Game/OAH/OAH_Blueprint/Player/ThirdPersonCharacter` OtherActor))
  (for _array_element (`/Game/OAH/OAH_Blueprint/Player/ThirdPersonCharacter.InventoryArray` _asthird_person_character) :!label _label_3
    (if (`KismetTextLibrary.EqualEqual_TextText` (`.ItemName_9_D15C36564F6449EF98FB6CB521D23004` (break `/Game/OAH/OAH_Blueprint/Player/InventorySystem/ItemStructure/Struct_ItemStruct` _array_element)) (`self.Mahjong_1`))
      (`self.KeyFound`)
      (`KismetSystemLibrary.PrintString` "You have the Dragon piece!")
      (bind _asthird_person_character_2 (cast `/Game/OAH/OAH_Blueprint/Player/ThirdPersonCharacter` (`GameplayStatics.GetPlayerCharacter` 0)))
      (`self.EnableInput` (`GameplayStatics.GetPlayerController` 0))
      (`/Game/OAH/OAH_Widget/HUDWidget.Show Door Text` (`/Game/OAH/OAH_Blueprint/Player/ThirdPersonCharacter.HUD` _asthird_person_character_2) true)
      (goto _label :!via `Open`))))

(event `KeyFound`
  ;[1 1 1] Locked Door
  (goto _label_3 :!via `Break`))

(event `self.collision_KeyCheck.OnComponentEndOverlap`
  (params (OverlappedComponent :type "PrimitiveComponent Object Reference") (OtherActor :type "Actor Object Reference") (OtherComp :type "PrimitiveComponent Object Reference") (OtherBodyIndex :type Integer))
  ;[1 1 1] Locked Door
  (cast `/Game/OAH/OAH_Blueprint/Player/ThirdPersonCharacter` OtherActor)
  (`self.DisableInput` (`GameplayStatics.GetPlayerController` 0) null)
  (`SceneComponent.SetVisibility` (`self.text_Locked`) false false)
  (bind _asthird_person_character (cast `/Game/OAH/OAH_Blueprint/Player/ThirdPersonCharacter` (`GameplayStatics.GetPlayerCharacter` 0)))
  (`/Game/OAH/OAH_Widget/HUDWidget.Show Door Text` (`/Game/OAH/OAH_Blueprint/Player/ThirdPersonCharacter.HUD` _asthird_person_character) false)
  (goto _label :!via `Close`))

(fn `UserConstructionScript`)