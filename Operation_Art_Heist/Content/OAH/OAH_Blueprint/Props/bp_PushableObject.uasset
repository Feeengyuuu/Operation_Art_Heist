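; Pushable block prop that the player shoves a set distance by walking into it head-on.
; On a hit it rounds the player's forward vector to a grid direction, then CanPush traces for facing, clearance, floor, objects on top and falling.
; If valid, it disables player movement, nudges them back, attaches them and plays a push montage.
; A timeline then slides the block, restoring walking and detaching the player when finished.
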(event `self.ReceiveHit`
  (params (MyComp :type "PrimitiveComponent Object Reference") (Other :type "Actor Object Reference") (OtherComp :type "PrimitiveComponent Object Reference") (bSelfMoved :type Boolean) (HitLocation :type "Vector Structure") (HitNormal :type "Vector Structure") (NormalImpulse :type "Vector Structure") (Hit :type "HitResult Structure (by ref)"))
  (bind _returnvalue (`self.GetActorForwardVector` Other))
  (bind _returnvalue_2 (`GameplayStatics.GetPlayerCharacter` 0))
  (bind _capsulecomponent (`Character.CapsuleComponent` _returnvalue_2))
  ;[1 1 1] Prepare to Push
  (if (== (`GameplayStatics.GetPlayerCharacter` 0) Other)
    (if (> (`KismetMathLibrary.Dot_VectorVector` HitNormal _returnvalue) 0.93)
      (set `self.pushableDirection` (`KismetMathLibrary.MakeVector` (`KismetMathLibrary.Conv_IntToDouble` (`KismetMathLibrary.Round` (.x _returnvalue))) (`KismetMathLibrary.Conv_IntToDouble` (`KismetMathLibrary.Round` (.y _returnvalue))) (`KismetMathLibrary.Conv_IntToDouble` (`KismetMathLibrary.Round` (.z _returnvalue)))))
      (bind _canpush (`self.canPush`))
      (if _canpush
        (`CharacterMovementComponent.DisableMovement` (`Character.CharacterMovement` _returnvalue_2))
        (`CapsuleComponent.SetCapsuleRadius` _capsulecomponent 35.0 true)
        (`KismetSystemLibrary.MoveComponentTo` _capsulecomponent (+ (`SceneComponent.K2_GetComponentLocation` _capsulecomponent) (* (`self.GetActorForwardVector` _returnvalue_2) -55.0)) (`SceneComponent.K2_GetComponentRotation` _capsulecomponent))
        (`self.K2_AttachToActor` (`GameplayStatics.GetPlayerCharacter` 0) self "None" "KeepWorld" "KeepWorld" "KeepWorld" true)
        (`|PlayMontage` (`Character.Mesh` (`GameplayStatics.GetPlayerCharacter` 0)) "/Game/OAH/OAH_CustomAnim/Pushing_UE_Montage.Pushing_UE_Montage" 3.0
          (:`then`
            (`self.Push`)))))))

(event `Push`
  ;[1 1 1] Block Movement
  (set `self.currentLocation` (`self.K2_GetActorLocation`))
  (bind (_direction _position) (`Timeline|MoveBlock` :!via `PlayFromStart`)
    (:`Update`
      (`self.K2_SetActorRelativeLocation` (+ (`self.currentLocation`) (* (* (`self.pushableDirection`) _position) (`self.travelDistance`)))))
    (:`Finished`
      (`self.StopPushing`))))

(event `StopPushing`
  (bind _returnvalue (`GameplayStatics.GetPlayerCharacter` 0))
  (bind _returnvalue_2 (`GameplayStatics.GetPlayerCharacter` 0))
  ;[1 1 1] Stop Pushing
  (`CapsuleComponent.SetCapsuleRadius` (`Character.CapsuleComponent` _returnvalue) 35.0 true)
  (`Character.StopAnimMontage` _returnvalue null)
  (`CharacterMovementComponent.SetMovementMode` (`Character.CharacterMovement` _returnvalue_2) "MOVE_Walking" 0)
  (`self.K2_DetachFromActor` _returnvalue_2 "KeepWorld" "KeepWorld" "KeepWorld"))

(fn `canPush`
  (returns (canPush :type Boolean))
  (locals (localCanPush :type Boolean :default true))
  (bind _returnvalue (`GameplayStatics.GetPlayerCharacter` 0))
  (bind _returnvalue_2 (`self.K2_GetActorLocation`))
  (bind _returnvalue_3 (`self.K2_GetActorLocation` _returnvalue))
  (bind _returnvalue_4 (+ (`self.K2_GetActorLocation`) (0.0 0.0 200.0)))
  (bind (_returnvalue_origin _returnvalue_boxextent) (`KismetMathLibrary.BreakBoxSphereBounds` (`StaticMesh.GetBounds` (`StaticMeshComponent.StaticMesh` (`self.PushableRock`)))))
  (bind _returnvalue_5 (+ (`self.K2_GetActorLocation`) (* (`self.pushableDirection`) (`self.travelDistance`)) (0.0 0.0 100.0)))
  (`|ExecutionSequence`
    (:`then_0`
      ;[1 1 1 1 50] 1. Check Player is facing box
      (bind (_outhit _returnvalue_6) (`KismetSystemLibrary.LineTraceSingle` _returnvalue_3 (+ _returnvalue_3 (* (`self.GetActorForwardVector` _returnvalue) 100.0)) "TraceTypeQuery1" false (`|MakeArray` _returnvalue :!type "Actor Object Reference") "None" false))
      (if _returnvalue_6
        (if (not (== (`.HitActor` (`GameplayStatics.BreakHitResult` _outhit)) self))
          (set `local.localCanPush` false))
        (else
          (set `local.localCanPush` false))))
    (:`then_1`
      ;[1 1 1 1 50] 2. Check is box have room to move
      (bind (_outhit_2 _returnvalue_7) (`KismetSystemLibrary.BoxTraceSingle` :`Start` (+ _returnvalue_2 (0.0 0.0 100.0)) :`End` (+ _returnvalue_2 (* (`self.pushableDirection`) (`self.travelDistance`)) (0.0 0.0 100.0)) :`HalfSize` (* _returnvalue_boxextent (`SceneComponent.RelativeScale3D` (`self.PushableRock`)) (0.9 0.9 0.9)) :`TraceChannel` "TraceTypeQuery1" :`DrawDebugType` "ForDuration"))
      (if (not (not _returnvalue_7))
        (set `local.localCanPush` false)))
    (:`then_2`
      ;[1 1 1 1 50] 3. Check if space has floor
      (bind (_outhit_3 _returnvalue_8) (`KismetSystemLibrary.LineTraceSingle` :`Start` _returnvalue_5 :`End` (+ _returnvalue_5 (0.0 0.0 -200.0)) :`TraceChannel` "TraceTypeQuery1" :`DrawDebugType` "ForDuration"))
      (if (not _returnvalue_8)
        (set `local.localCanPush` false)))
    (:`then_3`
      ;[1 1 1 1 50] 4. Check if there is anything on top of pushable
      (bind (_outhit_4 _returnvalue_9) (`KismetSystemLibrary.LineTraceSingle` :`Start` _returnvalue_4 :`End` (+ _returnvalue_4 (0.0 0.0 200.0)) :`TraceChannel` "TraceTypeQuery1" :`DrawDebugType` "ForDuration"))
      (if _returnvalue_9
        (set `local.localCanPush` false)))
    (:`then_4`
      ;[1 1 1 1 50] 5. Is Player falling
      (if (`NavMovementComponent.IsFalling` (`Character.CharacterMovement` (`GameplayStatics.GetPlayerCharacter` 0)))
        (set `local.localCanPush` false)))
    (:`then_5`
      (return (`local.localCanPush`)))))

(fn `UserConstructionScript`)