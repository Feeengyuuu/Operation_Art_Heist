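; Puddle prop that makes noise when the player moves quickly over it, raising an AI noise event.
; Each tick it checks whether player 0 overlaps it above a speed threshold, then plays a cracking wood cue at the player and reports noise at the puddle with the player as instigator.
; The stored sound instance blocks retriggering until a short delay stops and clears it.
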(event `self.ReceiveTick`
  (params (DeltaSeconds :type "Float (single-precision)"))
  (bind _returnvalue (`GameplayStatics.GetPlayerCharacter` 0))
  (if (`self.IsOverlappingActor` _returnvalue)
    (if (> (`KismetMathLibrary.VSize` (`self.GetVelocity` _returnvalue)) 300.0)
      (`self.soundInstance`
        (:`then`)
        (:`else`
          (bind _returnvalue_2 (`GameplayStatics.SpawnSoundAtLocation` "/Game/OAH/OAH_Audio/Audio_Prop/CrackingWoodCue_SFX.CrackingWoodCue_SFX" (`self.K2_GetActorLocation` (`GameplayStatics.GetPlayerCharacter` 0)) (struct) 1.0 1.0 0.0 null null))
          (set `self.soundInstance` _returnvalue_2)
          (`AISense_Hearing.ReportNoiseEvent` (`self.K2_GetActorLocation`) 1.0 (`GameplayStatics.GetPlayerCharacter` 0))
          (`KismetSystemLibrary.Delay` 0.5)
          (`AudioComponent.Stop` (`self.soundInstance`))
          (set `self.soundInstance` null))))))

(fn `UserConstructionScript`)