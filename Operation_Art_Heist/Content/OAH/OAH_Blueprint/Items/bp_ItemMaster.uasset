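; Master item Blueprint for a stealable world pickup with a value, driven by an ItemStats struct.
; BeginPlay displays the item's value on its text and records its world location as the origin position in ItemStats.
; Sphere overlap with ThirdPersonCharacter toggles input and the HUD steal prompt.
; Pressing E passes ItemStats to that character's PickUpItem, then destroys the item.
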(event `Key|E`
  (params (Key :type "Key Structure"))
  ;[1 1 1] Pick Up Item
  (:`Pressed`
    (bind _asthird_person_character (cast `/Game/OAH/OAH_Blueprint/Player/ThirdPersonCharacter` (stale `self.Sphere.OnComponentBeginOverlap` OtherActor)))
    (`/Game/OAH/OAH_Blueprint/Player/ThirdPersonCharacter.PickUpItem` _asthird_person_character (`self.itemStats`))
    (`self.K2_DestroyActor`)))

(event `self.Sphere.OnComponentBeginOverlap`
  (params (OverlappedComponent :type "PrimitiveComponent Object Reference") (OtherActor :type "Actor Object Reference") (OtherComp :type "PrimitiveComponent Object Reference") (OtherBodyIndex :type Integer) (bFromSweep :type Boolean) (SweepResult :type "HitResult Structure (by ref)"))
  ;[1 1 1] Pick Up Item
  (bind _asthird_person_character (cast `/Game/OAH/OAH_Blueprint/Player/ThirdPersonCharacter` OtherActor))
  (`self.EnableInput` (`GameplayStatics.GetPlayerController` 0))
  (`/Game/OAH/OAH_Widget/HUDWidget.ShowStealText` (`/Game/OAH/OAH_Blueprint/Player/ThirdPersonCharacter.HUD` _asthird_person_character) true))

(event `self.Sphere.OnComponentEndOverlap`
  (params (OverlappedComponent :type "PrimitiveComponent Object Reference") (OtherActor :type "Actor Object Reference") (OtherComp :type "PrimitiveComponent Object Reference") (OtherBodyIndex :type Integer))
  ;[1 1 1] Pick Up Item
  (bind _asthird_person_character (cast `/Game/OAH/OAH_Blueprint/Player/ThirdPersonCharacter` OtherActor))
  (`self.DisableInput` (`GameplayStatics.GetPlayerController` 0) null)
  (`/Game/OAH/OAH_Widget/HUDWidget.ShowStealText` (`/Game/OAH/OAH_Blueprint/Player/ThirdPersonCharacter.HUD` _asthird_person_character) false))

(event `self.ReceiveBeginPlay`
  (bind (_returnvalue_x _returnvalue_y _returnvalue_z) (`KismetMathLibrary.BreakVector` (`SceneComponent.K2_GetComponentLocation` (`self.DefaultSceneRoot`))))
  (bind (_itemstats_itemtype _itemstats_mesh _itemstats_itemname _itemstats_itemdescription _itemstats_itemvalue) (break `/Game/OAH/OAH_Blueprint/Player/InventorySystem/ItemStructure/Struct_ItemStruct` (`self.itemStats`)))
  ;[1 1 1] Show Value on Each Item and Get Original Pos of Each Item
  (`TextRenderComponent.K2_SetText` (`self.text_ItemValue`) (`KismetTextLibrary.Conv_DoubleToText` _itemstats_itemvalue "HalfToEven"))
  (`KismetMathLibrary.Vector_Set` (`.ItemOriginPosition_25_E22DB317429703BCA501A18A24C820B9` (break `/Game/OAH/OAH_Blueprint/Player/InventorySystem/ItemStructure/Struct_ItemStruct` (`self.itemStats`))) _returnvalue_x _returnvalue_y _returnvalue_z))

(fn `UserConstructionScript`)